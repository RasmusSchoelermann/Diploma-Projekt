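; Hunter_Unit is a unit Blueprint for the Hunter that supplies its own UI widget.
; GetWidged creates an E_Hunter_Range widget, passes it the selectable flag and a reference to the unit, initializes its health display from HP and MaxHP, and returns it.
; The event graph holds only disabled placeholder events, and the construction script just calls the parent.
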(fn `GetWidged`
  (params (`Can be selected` :type Boolean))
  (returns (NewParam :type "Widget Object Reference"))
  (bind _returnvalue (`|CreateWidget` "/Game/Nick_Tests/NickUi/E_Hunter_Range.E_Hunter_Range_C"))
  (set `/Game/Nick_Tests/NickUi/E_Hunter_Range.Can be Selected` `Can be selected` _returnvalue)
  (set `/Game/Nick_Tests/NickUi/E_Hunter_Range.Unit` self _returnvalue)
  (`/Game/Nick_Tests/NickUi/E_Hunter_Range.Update health` _returnvalue (`self.HP`) (`self.MaxHP`))
  (return _returnvalue))

(fn `UserConstructionScript`
  (`parent.UserConstructionScript`))