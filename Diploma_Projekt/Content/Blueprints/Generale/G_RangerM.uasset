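; G_RangerM is a unit Blueprint in the Generale folder for the RangerM unit, supplying that unit's UI widget.
; Its GetWidged function creates a RangerM_Widget, passes in the selectable flag and a reference to itself, initializes the health display from HP and MaxHP, then returns it.
; The event graph holds only disabled stubs, and the construction script just calls its parent.
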(fn `GetWidged`
  (params (`Can be selected` :type Boolean))
  (returns (NewParam :type "Widget Object Reference"))
  (bind _returnvalue (`|CreateWidget` "/Game/Blueprints/Generale/RangerM_Widget.RangerM_Widget_C"))
  (set `/Game/Blueprints/Generale/RangerM_Widget.Can be selected` `Can be selected` _returnvalue)
  (set `/Game/Blueprints/Generale/RangerM_Widget.Unit` self _returnvalue)
  (`/Game/Blueprints/Generale/RangerM_Widget.Update health` _returnvalue (`self.HP`) (`self.MaxHP`))
  (return _returnvalue))

(fn `UserConstructionScript`
  (`parent.UserConstructionScript`))